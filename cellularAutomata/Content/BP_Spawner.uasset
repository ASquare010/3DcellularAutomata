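; Spawner that runs a particle-life style simulation with white, red and yellow groups of BP_particle actors randomly placed within BoundSize.
; Each Tick, Rule applies inverse-distance-scaled pulls cyclically (white to red, red to yellow, yellow to white) using nested loops, then moves actors frame-rate dependently.
; ForceV is overwritten per pair rather than summed, so only the last counts.
; Velocity flips at hardcoded bounds independent of BoundSize; blue group logic is disconnected.
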(event `self.ReceiveBeginPlay`
  (bind _boundsize (`self.boundSize`))
  (bind _particlecount (`self.particleCount`))
  (`BoxComponent.SetBoxExtent` (`self.bound`) (`KismetMathLibrary.MakeVector` _boundsize _boundsize _boundsize) true)
  (`|ExecutionSequence`
    (:`then_0`
      (for _ (range 1 (+ _particlecount 1))
        (bind _returnvalue (`|SpawnActorFromClass` "/Game/BP_particle.BP_particle_C" (`self.getRandomTransform`) "Undefined" "MultiplyWithRoot" null null))
        (set `Actor.Tags` (`|MakeArray` "white" :!type "Name") _returnvalue)
        (`PrimitiveComponent.SetMaterial` (`/Game/BP_particle.particle` _returnvalue) 0 "/Game/Material/M_White.M_White")
        (`KismetArrayLibrary.Array_Add` (`self.whiteGroup`) _returnvalue)))
    (:`then_1`
      (for _ (range 1 (+ _particlecount 1))
        (bind _returnvalue_2 (`|SpawnActorFromClass` "/Game/BP_particle.BP_particle_C" (`self.getRandomTransform`) "Undefined" "MultiplyWithRoot" null null))
        (set `Actor.Tags` (`|MakeArray` "red" :!type "Name") _returnvalue_2)
        (`PrimitiveComponent.SetMaterial` (`/Game/BP_particle.particle` _returnvalue_2) 0 "/Game/Material/M_Red.M_Red")
        (`KismetArrayLibrary.Array_Add` (`self.redGroup`) _returnvalue_2)))
    (:`then_3`
      (for _ (range 1 (+ _particlecount 1))
        (bind _returnvalue_3 (`|SpawnActorFromClass` "/Game/BP_particle.BP_particle_C" (`self.getRandomTransform`) "Undefined" "MultiplyWithRoot" null null))
        (set `Actor.Tags` (`|MakeArray` "yellow" :!type "Name") _returnvalue_3)
        (`PrimitiveComponent.SetMaterial` (`/Game/BP_particle.particle` _returnvalue_3) 0 "/Game/Material/M_Yellow.M_Yellow")
        (`KismetArrayLibrary.Array_Add` (`self.yellowGroup`) _returnvalue_3)))))

(event `self.ReceiveTick`
  (params (DeltaSeconds :type "Float (single-precision)"))
  (`|ExecutionSequence`
    (:`then_0`
      (`self.rule` (`self.whiteGroup`) (`self.redGroup`) -10.0))
    (:`then_1`
      (`self.rule` (`self.redGroup`) (`self.yellowGroup`) -0.3))
    (:`then_2`
      (`self.rule` (`self.yellowGroup`) (`self.whiteGroup`) -0.1))))

(fn `getRandomLocation`
  (returns (loc :type "Vector Structure"))
  (bind _boundsize (`self.boundSize`))
  (bind _returnvalue (* -1.0 _boundsize))
  (return (`KismetMathLibrary.MakeVector` (`KismetMathLibrary.RandomFloatInRange` _returnvalue _boundsize) (`KismetMathLibrary.RandomFloatInRange` _returnvalue _boundsize) (`KismetMathLibrary.RandomFloatInRange` _returnvalue _boundsize))))

(fn `getRandomRotation`
  (returns (rot :type "Rotator Structure"))
  (return (`KismetMathLibrary.MakeRotator` (`KismetMathLibrary.RandomFloatInRange` 0.0 360.0) (`KismetMathLibrary.RandomFloatInRange` 0.0 360.0) (`KismetMathLibrary.RandomFloatInRange` 0.0 360.0))))

(fn `GetRandomScale`
  (returns (scale :type "Vector Structure"))
  (bind _returnvalue (`KismetMathLibrary.RandomFloatInRange` 1.0 1.4))
  (return (`KismetMathLibrary.MakeVector` _returnvalue _returnvalue _returnvalue)))

(fn `getRandomTransform`
  (returns (transform :type "Transform Structure"))
  (return (`KismetMathLibrary.MakeTransform` (`self.getRandomLocation`) (`self.getRandomRotation`) (`self.GetRandomScale`))))

(fn `rule`
  (params (particlesA :type "Array of /Game/BP_particle Object Reference") (particlesB :type "Array of /Game/BP_particle Object Reference") (g :type "Float (double-precision)"))
  (locals (force :type "Float (double-precision)") (forceV :type "Vector Structure") (gravity :type "Float (double-precision)"))
  (set `local.gravity` g)
  (for _array_element particlesA
    (set `local.forceV` (0.0 0.0 0.0))
    (for _array_element_2 particlesB
      (bind _returnvalue (`self.K2_GetActorLocation` _array_element))
      (bind _returnvalue_2 (`self.K2_GetActorLocation` _array_element_2))
      (bind _returnvalue_3 (`KismetMathLibrary.Vector_Distance` _returnvalue _returnvalue_2))
      (if (> _returnvalue_3 0.0)
        (set `local.force` (* (`local.gravity`) (/ 1.0 _returnvalue_3)))
        (set `local.forceV` (* (- _returnvalue _returnvalue_2) (`local.force`)))))
    (bind _output_get (set `/Game/BP_particle.velocity` (+ (`/Game/BP_particle.velocity` _array_element) (`local.forceV`)) _array_element))
    (`self.K2_SetActorLocation` _array_element (+ _output_get (`self.K2_GetActorLocation` _array_element)) false false)
    (`|ExecutionSequence`
      (:`then_0`
        (bind _x (.x (`self.K2_GetActorLocation` _array_element)))
        (if (or (< _x -5263.1) (> _x 5263.1))
          (bind (_velocity_x _velocity_y _velocity_z) (`KismetMathLibrary.BreakVector` (`/Game/BP_particle.velocity` _array_element)))
          (set `/Game/BP_particle.velocity` (`KismetMathLibrary.MakeVector` (* _velocity_x -1.0) _velocity_y _velocity_z) _array_element)))
      (:`then_1`
        (bind _y (.y (`self.K2_GetActorLocation` _array_element)))
        (if (or (< _y -5263.1) (> _y 5263.1))
          (bind (_velocity_x_2 _velocity_y_2 _velocity_z_2) (`KismetMathLibrary.BreakVector` (`/Game/BP_particle.velocity` _array_element)))
          (set `/Game/BP_particle.velocity` (`KismetMathLibrary.MakeVector` _velocity_x_2 (* _velocity_y_2 -1.0) _velocity_z_2) _array_element)))
      (:`then_2`
        (bind _z (.z (`self.K2_GetActorLocation` _array_element)))
        (if (or (< _z -5263.1) (> _z 5263.1))
          (bind (_velocity_x_3 _velocity_y_3 _velocity_z_3) (`KismetMathLibrary.BreakVector` (`/Game/BP_particle.velocity` _array_element)))
          (set `/Game/BP_particle.velocity` (`KismetMathLibrary.MakeVector` _velocity_x_3 _velocity_y_3 (* _velocity_z_3 -1.0)) _array_element))))))

(fn `UserConstructionScript`)